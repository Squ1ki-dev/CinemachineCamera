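; BP_ActorFollow is a camera actor that becomes the view target and follows the player on the X/Z plane using a dead zone.
; Tick tests four borders spaced symmetrically around the player's last recorded position.
; Crossing a border stops any current move, eases the Camera component toward the player via MoveComponentTo, then re-centres that axis's borders.
; Downward moves use a hardcoded duration instead of CameraMoveTime.
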(event `self.ReceiveBeginPlay`
  (set `self.Player` (`GameplayStatics.GetPlayerCharacter` 0))
  (`PlayerController.SetViewTargetWithBlend` (`GameplayStatics.GetPlayerController` 0) self 0.0 "VTBlend_Linear" 0.0 false)
  (`self.Update Dead Left Right Positions`)
  (`self.Update Dead Up Down Position`))

(event `self.ReceiveTick`
  (params (DeltaSeconds :type "Float (single-precision)"))
  (`self.Update Camera In Left Direction`)
  (`self.Update Camera In Right Direction`)
  (`self.Update Camera In Down Direction`)
  (`self.Update Camera In Up Direction`))

(event `Update Dead Left Right Positions`
  (bind _returnvalue_x (`KismetMathLibrary.BreakVector` (`self.K2_GetActorLocation` (`self.Player`))))
  (set `self.DeadPosRight` (+ _returnvalue_x (`self.BorderDistRight`)))
  (set `self.DeadPosLeft` (+ (* (`self.BorderDistRight`) -1.0) _returnvalue_x)))

(event `Update Dead Up Down Position`
  (bind (_returnvalue_x _returnvalue_y _returnvalue_z) (`KismetMathLibrary.BreakVector` (`self.K2_GetActorLocation` (`self.Player`))))
  (set `self.DeadPosUp` (+ _returnvalue_z (`self.BorderDistUp`)))
  (set `self.DeadPosDown` (+ _returnvalue_z (* (`self.BorderDistUp`) -1.0))))

(event `Update Camera In Right Direction`
  (bind (_returnvalue_x _returnvalue_y) (`KismetMathLibrary.BreakVector` (`self.K2_GetActorLocation`)))
  (bind _camera (`self.Camera`))
  (bind (_returnvalue_x_2 _returnvalue_y_2 _returnvalue_z) (`KismetMathLibrary.BreakVector` (`self.K2_GetActorLocation` (`self.Player`))))
  (if (>= _returnvalue_x_2 (`self.DeadPosRight`))
    (`|ExecutionSequence`
      (:`then_0`
        (`self.Camera Stop`)
        (`KismetSystemLibrary.MoveComponentTo` _camera (`KismetMathLibrary.InverseTransformLocation` (`self.GetTransform`) (`KismetMathLibrary.MakeVector` _returnvalue_x_2 _returnvalue_y _returnvalue_z)) (`SceneComponent.RelativeRotation` _camera) (`self.CameraEaseOut`) (`self.CameraEaseIn`) (`self.CameraMoveTime`)))
      (:`then_1`
        (`self.Update Dead Left Right Positions`)))))

(event `Update Camera In Left Direction`
  (bind (_returnvalue_x _returnvalue_y) (`KismetMathLibrary.BreakVector` (`self.K2_GetActorLocation`)))
  (bind _camera (`self.Camera`))
  (bind (_returnvalue_x_2 _returnvalue_y_2 _returnvalue_z) (`KismetMathLibrary.BreakVector` (`self.K2_GetActorLocation` (`self.Player`))))
  (if (<= _returnvalue_x_2 (`self.DeadPosLeft`))
    (`|ExecutionSequence`
      (:`then_0`
        (`self.Camera Stop`)
        (`KismetSystemLibrary.MoveComponentTo` _camera (`KismetMathLibrary.InverseTransformLocation` (`self.GetTransform`) (`KismetMathLibrary.MakeVector` _returnvalue_x_2 _returnvalue_y _returnvalue_z)) (`SceneComponent.RelativeRotation` _camera) (`self.CameraEaseOut`) (`self.CameraEaseIn`) (`self.CameraMoveTime`)))
      (:`then_1`
        (`self.Update Dead Left Right Positions`)))))

(event `Update Camera In Up Direction`
  (bind (_returnvalue_x _returnvalue_y) (`KismetMathLibrary.BreakVector` (`self.K2_GetActorLocation`)))
  (bind _camera (`self.Camera`))
  (bind (_returnvalue_x_2 _returnvalue_y_2 _returnvalue_z) (`KismetMathLibrary.BreakVector` (`self.K2_GetActorLocation` (`self.Player`))))
  (if (>= _returnvalue_z (`self.DeadPosUp`))
    (`|ExecutionSequence`
      (:`then_0`
        (`self.Camera Stop`)
        (`KismetSystemLibrary.MoveComponentTo` _camera (`KismetMathLibrary.InverseTransformLocation` (`self.GetTransform`) (`KismetMathLibrary.MakeVector` _returnvalue_x_2 _returnvalue_y _returnvalue_z)) (`SceneComponent.RelativeRotation` _camera) (`self.CameraEaseOut`) (`self.CameraEaseIn`) (`self.CameraMoveTime`)))
      (:`then_1`
        (`self.Update Dead Up Down Position`)))))

(event `Update Camera In Down Direction`
  (bind (_returnvalue_x _returnvalue_y) (`KismetMathLibrary.BreakVector` (`self.K2_GetActorLocation`)))
  (bind _camera (`self.Camera`))
  (bind (_returnvalue_x_2 _returnvalue_y_2 _returnvalue_z) (`KismetMathLibrary.BreakVector` (`self.K2_GetActorLocation` (`self.Player`))))
  (if (<= _returnvalue_z (`self.DeadPosDown`))
    (`|ExecutionSequence`
      (:`then_0`
        (`self.Camera Stop`)
        (`KismetSystemLibrary.MoveComponentTo` _camera (`KismetMathLibrary.InverseTransformLocation` (`self.GetTransform`) (`KismetMathLibrary.MakeVector` _returnvalue_x_2 _returnvalue_y _returnvalue_z)) (`SceneComponent.RelativeRotation` _camera) (`self.CameraEaseOut`) (`self.CameraEaseIn`) 0.5))
      (:`then_1`
        (`self.Update Dead Up Down Position`)))))

(event `Camera Stop`
  (`KismetSystemLibrary.MoveComponentTo` (`self.Camera`) :!via `Stop`))

(fn `UserConstructionScript`)